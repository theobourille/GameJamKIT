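; Car spawner actor that keeps traffic cycling by spawning random vehicles from CarArray at its root, yawed 180 degrees.
; BeginPlay spawns the first car after a short random delay.
; When a BP_VehicleBase overlaps EndCollision, SpawnCar waits a random delay, destroys it, prints a random index and spawns a replacement.
; A leftover force-push loop for the vehicle is disconnected and never runs.
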(event OnComponentBeginOverlap(EndCollision)
  (params (OverlappedComponent :type Primitive%20Component%20Object%20Reference) (OtherActor :type Actor%20Object%20Reference) (OtherComp :type Primitive%20Component%20Object%20Reference) (OtherBodyIndex :type Integer) (bFromSweep :type Boolean) (SweepResult :type Hit%20Result%20Structure%20%28by%20ref%29))
  (bind _asbp_vehicle_base (Utilities|Casting|CastToBP_VehicleBase OtherActor))
  (CallFunction|SpawnCar _asbp_vehicle_base))

(event Custom|SpawnCar
  (params (NewParam :type Actor%20Object%20Reference))
  (bind _cararray (Variables|Default|GetCarArray))
  (bind _returnvalue (Utilities|Array|LastIndex _cararray))
  (bind _returnvalue_2 (Math|Random|RandomIntegerinRange 0 _returnvalue))
  (Utilities|FlowControl|Delay (Math|Random|RandomFloatinRange 0.0 2.0))
  (bind _asbp_vehicle_base (Utilities|Casting|CastToBP_VehicleBase NewParam))
  (Actor|DestroyActor _asbp_vehicle_base)
  (Development|PrintString (Utilities|String|ToString(Integer) _returnvalue_2))
  (Game|SpawnActorfromClass (Utilities|Array|Get(acopy) _cararray _returnvalue_2) (CallFunction|GetRotationVehicule (Variables|Default|GetDefaultSceneRoot)) "AlwaysSpawn" 0 0))

(event EventBeginPlay
  (bind _cararray (Variables|Default|GetCarArray))
  (Utilities|FlowControl|Delay (Math|Random|RandomFloatinRange 0.0 2.0))
  (Game|SpawnActorfromClass (Utilities|Array|Get(acopy) _cararray (Math|Random|RandomIntegerinRange 0 (Utilities|Array|LastIndex _cararray))) (CallFunction|GetRotationVehicule (Variables|Default|GetDefaultSceneRoot)) "AlwaysSpawn" 0 0))

(event Collision|EventActorBeginOverlap
  (params (OtherActor :type Actor%20Object%20Reference)))

(event EventTick
  (params (DeltaSeconds :type Float%20%28single-precision%29)))

(fn ConstructionScript)

(fn GetRotationVehicule
  (params (self2 :type Scene%20Component%20Object%20Reference))
  (bind _returnvalue (Transformation|GetWorldTransform self2))
  (return (Math|Transform|MakeTransform (.location _returnvalue) (Math|Rotator|MakeRotator (.roll (.rotation _returnvalue)) (.pitch (.rotation _returnvalue)) (+ (.yaw (.rotation _returnvalue)) 1.8e+02)) (.scale _returnvalue))))