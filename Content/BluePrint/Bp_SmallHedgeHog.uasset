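; Baby hedgehog character that joins the player's mother hedgehog on sphere overlap and follows her in formation.
; Every tick it pathfinds to its ID's slot in the mother's mesh space, walking or running by her in-line state.
; Vehicle hits launch and kill assigned, in-line babies, shifting higher IDs down to close the gap.
; It also eats collectables to raise the mother's capacity count, and snaps to traced ground on first tick.
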(event OnComponentBeginOverlap(Sphere)
  (params (OverlappedComponent :type Primitive%20Component%20Object%20Reference) (OtherActor :type Actor%20Object%20Reference) (OtherComp :type Primitive%20Component%20Object%20Reference) (OtherBodyIndex :type Integer) (bFromSweep :type Boolean) (SweepResult :type Hit%20Result%20Structure%20%28by%20ref%29))
  (bind _mother (Variables|Default|GetMother))
  (bind _assignedbaby (Variables|/Game/BluePrint/Bp_MotherHedgeHog.BP_MotherHedgeHog_C|GetAssignedBaby _mother))
  ;[1 1 1] MOTHER GATHERING
  (if (== OtherActor _mother)
    (Physics|SetSimulatePhysics (Variables|Collision|GetCapsuleComponent) false)
    (if (not (Variables|Default|GetAssigned))
      (Variables|Default|SetID _assignedbaby)
      (Math|Integer|IncrementInt _assignedbaby
        (:%20%20
          (Variables|Default|SetAssigned true)
          (Audio|PlaySoundatLocation "/Game/Sounds/HEDGEHOGS/Happy_AM_Cue.Happy_AM_Cue" (Transformation|GetActorLocation) "0, 0, 0" 1.0 1.0 0.0 "/Game/Sounds/AttenuationSettings/SA_DeathAttenuation.SA_DeathAttenuation" 0 0)
          (Rendering|SetVisibility (Variables|Default|GetShield) false false))))))

(event OnComponentBeginOverlap(Mesh)
  (params (OverlappedComponent :type Primitive%20Component%20Object%20Reference) (OtherActor :type Actor%20Object%20Reference) (OtherComp :type Primitive%20Component%20Object%20Reference) (OtherBodyIndex :type Integer) (bFromSweep :type Boolean) (SweepResult :type Hit%20Result%20Structure%20%28by%20ref%29))
  ;[1 1 1] MANAGE VEHICULE COLLISION
  (Utilities|FlowControl|Sequence
    (:then_0
      (bind _asbp_vehicle_base (Utilities|Casting|CastToBP_VehicleBase OtherActor))
      (if (Variables|Default|GetAssigned)
        (if (Variables|Default|GetIsInLine)
          (Variables|Default|SetAssigned false)
          (Physics|SetSimulatePhysics (Variables|Collision|GetCapsuleComponent) true)
          (Physics|AddImpulse (Variables|Collision|GetCapsuleComponent) (* (Math|Vector|MakeVector (Math|Random|RandomFloatinRange 0.0 0.1) (CallFunction|GetVehiculeDirection _asbp_vehicle_base) (Math|Random|RandomFloatinRange 0.0 0.1)) 7e+02) "None" true)
          (CallFunction|ManageReplacement)
          (Audio|PlaySoundatLocation "/Game/Sounds/HEDGEHOGS/SC_HedgeHog_Death.SC_HedgeHog_Death" (Transformation|GetActorLocation) "0, 0, 0" 1.0 1.0 0.0 "/Game/Sounds/AttenuationSettings/SA_DeathAttenuation.SA_DeathAttenuation" 0 0)
          (Utilities|FlowControl|Delay 2.0)
          (Actor|DestroyActor))))
    (:then_1
      ;[1 1 1] Collectables
      (bind _asbp_collectable_base (Utilities|Casting|CastToBP_CollectableBase OtherActor))
      (bind _asbp_mother_hedge_hog (Utilities|Casting|CastToBP_MotherHedgeHog (Game|Player|GetPlayerPawn 0)))
      (Math|Integer|IncrementInt (Variables|/Game/BluePrint/Bp_MotherHedgeHog.BP_MotherHedgeHog_C|GetCapacityCount _asbp_mother_hedge_hog)
        (:%20%20
          (Audio|PlaySoundatLocation "/Game/Sounds/BUGS/Bug_Crunch_AM_Cue.Bug_Crunch_AM_Cue" (Transformation|GetActorLocation) "0, 0, 0" 1.0 1.0 0.0 "/Game/Sounds/AttenuationSettings/SA_DeathAttenuation.SA_DeathAttenuation" 0 0)
          (Actor|DestroyActor _asbp_collectable_base))))))

(event EventBeginPlay
  ;[1 1 1] BEGINPLAY
  (bind _returnvalue (Actor|GetActorOfClass "/Game/BluePrint/bp_CarSpawner.Bp_CarSpawner_C")))

(event EventTick
  (params (DeltaSeconds :type Float%20%28single-precision%29))
  (bind _returnvalue (CallFunction|CreateTransformedDestination))
  (bind _charactermovement (Variables|Character|GetCharacterMovement))
  ;[1 1 1] TICK EVENT
  (Utilities|FlowControl|Sequence
    (:then_0
      ;[1 1 1] SpawnAndGetMother
      (Utilities|FlowControl|DoOnce false
        (:Completed
          (CallFunction|DecalHerissons)
          (bind _asbp_mother_hedge_hog (Utilities|Casting|CastToBP_MotherHedgeHog (Game|Player|GetPlayerPawn 0)))
          (Variables|Default|SetMother _asbp_mother_hedge_hog)
          (Development|PrintString "Grounded"))))
    (:then_1
      ;[1 1 1] SetAlignmentBoolean
      (Variables|Default|SetIsInLine (Variables|/Game/BluePrint/Bp_MotherHedgeHog.BP_MotherHedgeHog_C|GetIsInLine (Variables|Default|GetMother))))
    (:then_2
      ;[1 1 1] MoveBabyToHisPosition
      (if (Variables|Default|GetAssigned)
        (AI|AIMoveTo self _returnvalue 0 5.0 false
          (:then
            (Transformation|SetActorRotation (Math|Rotator|MakeRotator 0.0 0.0 (+ (.yaw (Math|Rotator|FindLookatRotation (Transformation|GetActorLocation) _returnvalue)) -9e+01)))
            (Collision|IgnoreActorwhenMoving (Variables|Collision|GetCapsuleComponent) (Game|GetPlayerCharacter 0) true)))))
    (:then_3
      ;[1 1 1] SetSpeedFromAllignment
      (if (Variables|Default|GetIsInLine)
        (Variables|/Script/Engine.CharacterMovementComponent|SetMaxWalkSpeed _charactermovement (Variables|Default|GetWalkSpeed))
        (else
          (Variables|/Script/Engine.CharacterMovementComponent|SetMaxWalkSpeed _charactermovement (Variables|Default|GetRunSpeed)))))))

(fn ConstructionScript)

(fn DecalHerissons
  (bind _capsulecomponent (Variables|Collision|GetCapsuleComponent))
  (bind _returnvalue (Transformation|GetWorldLocation _capsulecomponent))
  (bind (_x _y _z) (Math|Vector|BreakVector _returnvalue))
  (bind _outhit (Collision|LineTraceByChannel _returnvalue (Math|Vector|MakeVector _x _y (- _z (Variables|Default|GetLineTraceDistance))) "TraceTypeQuery1" false 0 "ForDuration" true "(R=1.000000,G=0.000000,B=0.000000,A=1.000000)" "(R=0.000000,G=1.000000,B=0.000000,A=1.000000)" 1.0))
  (if (Class|KismetMathLibrary|NotEqualExactlyVectorVector (.Location (Collision|BreakHitResult _outhit)) "0, 0, 0")
    (Transformation|SetActorLocation (.Location (Collision|BreakHitResult _outhit)) false false)))

(fn CreateTransformedDestination
  (return (Math|Transform|TransformLocation (Transformation|GetWorldTransform (Variables|/Game/BluePrint/Bp_MotherHedgeHog.BP_MotherHedgeHog_C|GetSkeletalMesh (Variables|Default|GetMother))) (Utilities|Array|Get(acopy) (Variables|/Game/BluePrint/Bp_MotherHedgeHog.BP_MotherHedgeHog_C|GetActualPositionArray (Variables|Default|GetMother)) (Variables|Default|GetID)))))

(fn GetVehiculeDirection
  (params (Vehicule :type BP%20Vehicle%20Base%20Object%20Reference))
  (return (.y (Math|Vector|Normalize (Transformation|GetComponentVelocity (Variables|/Game/BluePrint/Cars/BP_VehicleBase.BP_VehicleBase_C|GetVehicle Vehicule))))))

(fn ManageReplacement
  (Math|Integer|DecrementInt (Variables|/Game/BluePrint/Bp_MotherHedgeHog.BP_MotherHedgeHog_C|GetAssignedBaby (Variables|Default|GetMother))
    (:%20%20
      (bind _outactors (Actor|GetAllActorsOfClass "Bp_SmallHedgeHog_C"))
      (for _array_element _outactors
        (if (> (Variables|Bp_SmallHedgeHog_C|GetID _array_element) (Variables|Default|GetID))
          (Math|Integer|DecrementInt (Variables|Bp_SmallHedgeHog_C|GetID _array_element)))))))