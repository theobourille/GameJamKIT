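; Hedgehog spawner actor that populates a box area around itself with instances of a configurable class when play begins.
; BeginPlay picks a random count, then loops to spawn each actor at a random point inside the box extent with a random yaw.
; A debug box draw for the spawn area is present but not connected to any event.
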(event EventBeginPlay
  (bind _output_get (Variables|Default|SetMaxHedgeHoginnumber (Math|Random|RandomIntegerinRange 6 10)))
  (bind _result (Math|Integer|DecrementInt _output_get)
    (:%20%20
      (for _index (range 0 _result)
        (Game|SpawnActorfromClass (Variables|Default|GetClassToSpawn) (Math|Transform|MakeTransform (Math|Random|RandomPointinBoundingBox (.location (Transformation|GetWorldTransform (Variables|Default|GetDefaultSceneRoot))) (Variables|Default|GetBox)) (Math|Rotator|MakeRotator 0.0 0.0 (Math|Random|RandomFloatinRange -3.6e+02 3.6e+02)) "1,1,1") "Undefined" 0 0)))))

(event Collision|EventActorBeginOverlap
  (params (OtherActor :type Actor%20Object%20Reference)))

(event EventTick
  (params (DeltaSeconds :type Float%20%28single-precision%29)))

(fn ConstructionScript)