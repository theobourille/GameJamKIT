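; BP_EndLEvel is the level-end trigger that finishes the game when the player's mother hedgehog enters its box.
; On overlap it sets the mother's in-line flag, calls its circle/linear formation switch and plays a victory sound.
; It replaces all widgets with WBP_GameOver under UI-only mouse input.
; It also loops over small hedgehogs, using an index-based Delay intended to stagger happy sounds from living, assigned ones.
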(event OnComponentBeginOverlap(Box)
  (params (OverlappedComponent :type Primitive%20Component%20Object%20Reference) (OtherActor :type Actor%20Object%20Reference) (OtherComp :type Primitive%20Component%20Object%20Reference) (OtherBodyIndex :type Integer) (bFromSweep :type Boolean) (SweepResult :type Hit%20Result%20Structure%20%28by%20ref%29))
  (bind _returnvalue (Game|GetPlayerController 0))
  (bind _motherref (Variables|Default|GetMotherRef))
  (if (== OtherActor _motherref)
    (Variables|/Game/BluePrint/Bp_MotherHedgeHog.BP_MotherHedgeHog_C|SetIsInLine _motherref true)
    (Default|SwitchBetweenCircleLinear _motherref)
    (Audio|PlaySound2D "/Game/Sounds/Victory_AM.Victory_AM" 1.5 1.0 0.0 0 0)
    ;[1 1 1] EndGameHUD
    (Viewport|RemoveAllWidgets)
    (bind _returnvalue_2 (UserInterface|CreateWidget "/Game/BluePrint/Widget/WBP_GameOver.WBP_GameOver_C" _returnvalue))
    (Input|SetInputModeUIOnly _returnvalue _returnvalue_2 "DoNotLock")
    (UserInterface|Viewport|AddtoViewport _returnvalue_2 0)
    (Variables|/Script/Engine.PlayerController|SetbShowMouseCursor _returnvalue true)
    (Variables|/Script/Engine.PlayerController|SetbEnableClickEvents _returnvalue true)
    ;[1 1 1] HedgeHogsScream
    (bind _outactors (Actor|GetAllActorsOfClass "/Game/BluePrint/Bp_SmallHedgeHog.Bp_SmallHedgeHog_C"))
    (for (_array_element _array_index) _outactors
      (|PlaySoundForHedgeHogs_2 _array_element _array_index))))

(event EventBeginPlay
  (bind _asbp_mother_hedge_hog (Utilities|Casting|CastToBP_MotherHedgeHog (Game|Player|GetPlayerPawn 0)))
  (Variables|Default|SetMotherRef _asbp_mother_hedge_hog))

(fn ConstructionScript)